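; Paint can actor that paints on easel canvases wherever an on-screen Pointer widget aims.
; While IsPainting is set, Tick deprojects the pointer's position and runs a complex visibility line trace; otherwise it restores game-only input.
; Hits on actors matching four hardcoded Easel_BP display names send the collision UV to PaintOnCanvas and clear IsRumble.
; Hits on other actors set IsRumble.
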(event `self.ReceiveBeginPlay`
  (bind _asbp_first_person_character (cast `/Game/FirstPerson/Blueprints/BP_FirstPersonCharacter` (`GameplayStatics.GetPlayerCharacter` 0)))
  (set `self.As BP First Person Character` _asbp_first_person_character)
  (bind _outactors (`GameplayStatics.GetAllActorsOfClass` "/Game/BluePrints/Easel_BP.Easel_BP_C"))
  (set `self.easelBP` (`|GetArrayItem` _outactors)))

(event `self.ReceiveTick`
  (params (DeltaSeconds :type "Float (single-precision)"))
  (if (`self.isPainting`)
    (bind _foundwidgets (`WidgetBlueprintLibrary.GetAllWidgetsOfClass` "/Game/Widget/Pointer.Pointer_C"))
    (set `self.Pointer` (`|GetArrayItem` _foundwidgets))
    (`self.TraceLine`)
    (else
      (`WidgetBlueprintLibrary.SetInputMode_GameOnly` (`GameplayStatics.GetPlayerController` 0)))))

(fn `TraceLine`
  (bind _pointer (`self.Pointer`))
  (bind (_worldlocation _worlddirection) (`PlayerController.DeprojectScreenPositionToWorld` (`GameplayStatics.GetPlayerController` 0) (`/Game/Widget/Pointer.NormX` _pointer) (`/Game/Widget/Pointer.NormY` _pointer)))
  (bind (_outhit _returnvalue) (`KismetSystemLibrary.LineTraceSingle` _worldlocation (+ _worldlocation (* _worlddirection 10000000000.0)) "TraceTypeQuery1" true (`|MakeArray` (cast `/Game/VRTemplate/Blueprints/VRPawn` (`GameplayStatics.GetPlayerPawn` 0) :!pure true) :!type "Actor Object Reference") "ForOneFrame"))
  (if _returnvalue
    (bind (_bblockinghit _binitialoverlap _time _distance _location _impactpoint _normal _impactnormal _physmat _hitactor) (`GameplayStatics.BreakHitResult` _outhit))
    (bind _returnvalue_2 (`KismetSystemLibrary.GetDisplayName` _hitactor))
    (if (or (`KismetStringLibrary.EqualEqual_StrStr` _returnvalue_2 "Easel_BP") (`KismetStringLibrary.EqualEqual_StrStr` _returnvalue_2 "Easel_BP2") (`KismetStringLibrary.EqualEqual_StrStr` _returnvalue_2 "Easel_BP3") (`KismetStringLibrary.EqualEqual_StrStr` _returnvalue_2 "Easel_BP4"))
      (set `self.IsRumble` false)
      (bind _aseasel_bp (cast `/Game/BluePrints/Easel_BP` _hitactor))
      (`/Game/BluePrints/Easel_BP.PaintOnCanvas` _aseasel_bp (`GameplayStatics.FindCollisionUV` _outhit))
      (else
        (set `self.IsRumble` true)))
    (else
      (`KismetSystemLibrary.PrintString` "no hit"))))

(fn `UserConstructionScript`)